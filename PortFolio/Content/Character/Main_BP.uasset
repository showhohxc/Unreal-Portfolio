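; Main character Blueprint that holds debug key bindings for player stats and pickup locations.
; Pressing R lowers health and stamina by a fixed amount and adds a coin, with no clamping.
; Pressing P calls ShowPickupLocations, whose body is not defined in these graphs.
; BeginPlay, overlap, Tick and the construction script are empty.
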(event EventBeginPlay)

(event Collision|EventActorBeginOverlap
  (params (OtherActor :type Actor%20Object%20Reference)))

(event EventTick
  (params (DeltaSeconds :type Float%20%28single-precision%29)))

(event Input|KeyboardEvents|R
  (params (Key :type Key%20Structure :default "None"))
  (:Pressed
    (Variables|Default|SetfHealth (- (Variables|Default|GetfHealth) 5.0))
    (Variables|Default|SetfStamina (- (Variables|Default|GetfStamina) 5.0))
    (Variables|Default|SetnCoins (+ (Variables|Default|GetnCoins) 1))))

(event Input|KeyboardEvents|P
  (params (Key :type Key%20Structure :default "None"))
  (:Pressed
    (Class|Main|ShowPickupLocations)))

(fn ConstructionScript)